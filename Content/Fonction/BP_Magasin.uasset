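; BP_Magasin is a small Blueprint that prints French greetings and a fruit shop inventory to the screen.
; On BeginPlay it calls the DireBonjour custom event, which waits briefly and then prints "Bonjour".
; The Magasin function prints a welcome and the given pear, apple and banana counts, then returns their total.
; Nothing in this file calls Magasin, and the construction script is empty.
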(event Custom|Dire%20Bonjour
  (Utilities|FlowControl|Delay 2.0)
  (Development|PrintString "Bonjour"))

(event EventBeginPlay
  (CallFunction|DireBonjour))

(fn ConstructionScript)

(fn Magasin
  (params (Poire :type Integer) (Pomme :type Integer) (Banane :type Integer))
  (Development|PrintString "Bienvenue dans le magasin" true true "(R=0.000000,G=0.660000,B=1.000000,A=1.000000)" 5.0)
  (Development|PrintString (Utilities|String|Append (Utilities|String|Append "Il y a " (Utilities|String|ToString(Integer) Poire)) " poires") true true "(R=0.000000,G=0.660000,B=1.000000,A=1.000000)" 5.0)
  (Development|PrintString (Utilities|String|Append (Utilities|String|Append "Il y a " (Utilities|String|ToString(Integer) Pomme)) " pommes ") true true "(R=0.000000,G=0.660000,B=1.000000,A=1.000000)" 5.0)
  (Development|PrintString (Utilities|String|Append (Utilities|String|Append "Il y a " (Utilities|String|ToString(Integer) Banane)) " bannanes") true true "(R=0.000000,G=0.660000,B=1.000000,A=1.000000)" 5.0)
  (return (+ Poire Pomme Banane)))